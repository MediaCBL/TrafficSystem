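; Base four-way intersection actor that alternates green and red between North-South and East-West traffic.
; On BeginPlay it sorts its child-actor traffic signals and lane actors into per-axis arrays and starts a looping timer.
; Each tick of that timer flip-flops the priority, and SwitchLanePriority sets both lights and lanes, with opposite directions sharing one branch.
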(event Custom|ChangeLanePriority
  (Utilities|FlowControl|FlipFlop
    (:A
      (CallFunction|SwitchLanePriority "North"))
    (:B
      (CallFunction|SwitchLanePriority "East"))))

(event EventBeginPlay
  (CallFunction|SetLaneRef)
  (Utilities|Time|SetTimerbyEvent (delegate Custom|ChangeLanePriority) (Variables|Default|GetChangeLanePriorityDelay) true)
  ;[0.15 0.15 0.15 0.5] Initialize signals one time before timer start
  (CallFunction|SwitchLanePriority "North")
  (CallFunction|SwitchLanePriority "South")
  (CallFunction|SwitchLanePriority "East")
  (CallFunction|SwitchLanePriority "West"))

(fn ConstructionScript)

(fn SetLaneRef
  (Utilities|FlowControl|Sequence
    (:then_0
      (bind _asbp_traffic_signal_base (Utilities|Casting|CastToBP_TrafficSignalBase (Variables|/Script/Engine.ChildActorComponent|GetChildActor (Variables|Default|GetTrafficLight1)))
        (:then
          (Utilities|Array|AddUnique (Variables|Default|GetNorthSouthLights) _asbp_traffic_signal_base))
        (:CastFailed
          _))
      (bind _asbp_traffic_signal_base_2 (Utilities|Casting|CastToBP_TrafficSignalBase (Variables|/Script/Engine.ChildActorComponent|GetChildActor (Variables|Default|GetTrafficLight4))))
      (Utilities|Array|AddUnique (Variables|Default|GetNorthSouthLights) _asbp_traffic_signal_base_2))
    (:then_1
      (bind _asbp_traffic_signal_base_3 (Utilities|Casting|CastToBP_TrafficSignalBase (Variables|/Script/Engine.ChildActorComponent|GetChildActor (Variables|Default|GetTrafficLight2)))
        (:then
          (Utilities|Array|AddUnique (Variables|Default|GetEastWestLights) _asbp_traffic_signal_base_3))
        (:CastFailed
          _))
      (bind _asbp_traffic_signal_base_4 (Utilities|Casting|CastToBP_TrafficSignalBase (Variables|/Script/Engine.ChildActorComponent|GetChildActor (Variables|Default|GetTrafficLight3))))
      (Utilities|Array|AddUnique (Variables|Default|GetEastWestLights) _asbp_traffic_signal_base_4))
    (:then_2
      (bind _asbp_traffic_lane_actor (Utilities|Casting|CastToBP_TrafficLaneActor (Variables|/Script/Engine.ChildActorComponent|GetChildActor (Variables|Default|GetTrafficLane1)))
        (:then
          (Utilities|Array|AddUnique (Variables|Default|GetNorthSouthLane) _asbp_traffic_lane_actor))
        (:CastFailed
          _))
      (bind _asbp_traffic_lane_actor_2 (Utilities|Casting|CastToBP_TrafficLaneActor (Variables|/Script/Engine.ChildActorComponent|GetChildActor (Variables|Default|GetTrafficLane4))))
      (Utilities|Array|AddUnique (Variables|Default|GetNorthSouthLane) _asbp_traffic_lane_actor_2))
    (:then_3
      (bind _asbp_traffic_lane_actor_3 (Utilities|Casting|CastToBP_TrafficLaneActor (Variables|/Script/Engine.ChildActorComponent|GetChildActor (Variables|Default|GetTrafficLane2)))
        (:then
          (Utilities|Array|AddUnique (Variables|Default|GetEastWestLane) _asbp_traffic_lane_actor_3))
        (:CastFailed
          _))
      (bind _asbp_traffic_lane_actor_4 (Utilities|Casting|CastToBP_TrafficLaneActor (Variables|/Script/Engine.ChildActorComponent|GetChildActor (Variables|Default|GetTrafficLane3))))
      (Utilities|Array|AddUnique (Variables|Default|GetEastWestLane) _asbp_traffic_lane_actor_4))))

(fn SwitchLanePriority
  (params (LaneOrientationPriority :type ETrafficLaneOrientation%20Enum :default "North"))
  (switch Utilities|FlowControl|Switch|SwitchonETrafficLaneOrientation LaneOrientationPriority
    (:North
      (Utilities|FlowControl|Sequence :!label _label
        (:then_0
          (for _array_element (Variables|Default|GetNorthSouthLights)
            (Class|TrafficSignalActor|SetSignalState _array_element "Green"))
          (for _array_element_2 (Variables|Default|GetEastWestLights)
            (Class|TrafficSignalActor|SetSignalState _array_element_2 "Red")))
        (:then_1
          (for _array_element_3 (Variables|Default|GetNorthSouthLane)
            (Class|TrafficLaneActor|SetState _array_element_3 "Green"))
          (for _array_element_4 (Variables|Default|GetEastWestLane)
            (Class|TrafficLaneActor|SetState _array_element_4 "Red")))))
    (:South
      (goto _label))
    (:East
      (Utilities|FlowControl|Sequence :!label _label_2
        (:then_0
          (for _array_element_5 (Variables|Default|GetNorthSouthLights)
            (Class|TrafficSignalActor|SetSignalState _array_element_5 "Red"))
          (for _array_element_6 (Variables|Default|GetEastWestLights)
            (Class|TrafficSignalActor|SetSignalState _array_element_6 "Green")))
        (:then_1
          (for _array_element_7 (Variables|Default|GetNorthSouthLane)
            (Class|TrafficLaneActor|SetState _array_element_7 "Red"))
          (for _array_element_8 (Variables|Default|GetEastWestLane)
            (Class|TrafficLaneActor|SetState _array_element_8 "Green")))))
    (:West
      (goto _label_2))))