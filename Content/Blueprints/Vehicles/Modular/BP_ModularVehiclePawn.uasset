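; BP_ModularVehiclePawn is a player-driven modular vehicle pawn that turns Enhanced Input into vehicle simulation inputs and camera control.
; On possession it adds the vehicle input mapping context for the player controller.
; Steering, throttle, brake, handbrake and reverse actions feed named inputs on the VehicleSimComponent, with steering combined and the rest overriding.
; Camera input rotates the spring arm by mouse sensitivity, with pitch clamped.
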(event Input|EnhancedActionEvents|EnhancedInputActionIA_Throttle
  (params (ActionValue :type Float%20%28double-precision%29) (ElapsedSeconds :type Float%20%28double-precision%29) (TriggeredSeconds :type Float%20%28double-precision%29) (InputAction :type Input%20Action%20Object%20Reference :default "/TrafficSystem/Inputs/IA_Throttle.IA_Throttle"))
  (Class|ModularVehicleBaseComponent|SetInputAxis1D (Variables|Default|GetVehicleSimComponent) "Throttle" ActionValue "Override"))

(event Input|EnhancedActionEvents|EnhancedInputActionIA_Steering
  (params (ActionValue :type Float%20%28double-precision%29) (ElapsedSeconds :type Float%20%28double-precision%29) (TriggeredSeconds :type Float%20%28double-precision%29) (InputAction :type Input%20Action%20Object%20Reference :default "/TrafficSystem/Inputs/IA_Steering.IA_Steering"))
  (Class|ModularVehicleBaseComponent|SetInputAxis1D (Variables|Default|GetVehicleSimComponent) "Steering" ActionValue "Combine"))

(event Input|EnhancedActionEvents|EnhancedInputActionIA_Brake
  (params (ActionValue :type Float%20%28double-precision%29) (ElapsedSeconds :type Float%20%28double-precision%29) (TriggeredSeconds :type Float%20%28double-precision%29) (InputAction :type Input%20Action%20Object%20Reference :default "/TrafficSystem/Inputs/IA_Brake.IA_Brake"))
  (Class|ModularVehicleBaseComponent|SetInputAxis1D (Variables|Default|GetVehicleSimComponent) "Brake" ActionValue "Override"))

(event Input|EnhancedActionEvents|EnhancedInputActionIA_Handbrake
  (params (ActionValue :type Boolean) (ElapsedSeconds :type Float%20%28double-precision%29) (TriggeredSeconds :type Float%20%28double-precision%29) (InputAction :type Input%20Action%20Object%20Reference :default "/TrafficSystem/Inputs/IA_Handbrake.IA_Handbrake"))
  (Class|ModularVehicleBaseComponent|SetInputBool (Variables|Default|GetVehicleSimComponent) "Handbrake" ActionValue "Override"))

(event Input|EnhancedActionEvents|EnhancedInputActionIA_Reverse
  (params (ActionValue :type Boolean) (ElapsedSeconds :type Float%20%28double-precision%29) (TriggeredSeconds :type Float%20%28double-precision%29) (InputAction :type Input%20Action%20Object%20Reference :default "/TrafficSystem/Inputs/IA_Reverse.IA_Reverse"))
  (Class|ModularVehicleBaseComponent|SetInputBool (Variables|Default|GetVehicleSimComponent) "Reverse" ActionValue "Override"))

(event Input|EnhancedActionEvents|EnhancedInputActionIA_CameraRotation
  (params (ActionValue :type Vector%202D%20Structure) (ElapsedSeconds :type Float%20%28double-precision%29) (TriggeredSeconds :type Float%20%28double-precision%29) (InputAction :type Input%20Action%20Object%20Reference :default "/TrafficSystem/Inputs/IA_CameraRotation.IA_CameraRotation"))
  (bind _springarm (Variables|Default|GetSpringArm))
  (bind _relativerotation (Variables|/Script/Engine.SceneComponent|GetRelativeRotation _springarm))
  (:Triggered
    (Transformation|SetRelativeRotation (Variables|Default|GetSpringArm) (Math|Rotator|MakeRotator 0.0 (Math|Float|Clamp(Float) (+ (* (.y ActionValue) (Variables|Default|GetMouseSensivity)) (.pitch _relativerotation)) -8e+01 8e+01) (+ (* (* (.x ActionValue) (Variables|Default|GetMouseSensivity)) -1.0) (.yaw _relativerotation))) false false)))

(event EventPossessed
  (params (NewController :type Controller%20Object%20Reference))
  (bind _asplayer_controller (Utilities|Casting|CastToPlayerController (Pawn|GetController)))
  (Input|AddMappingContext (PlayerController|LocalPlayerSubsystems|GetEnhancedInputLocalPlayerSubsystem _asplayer_controller) "/TrafficSystem/Inputs/IMC_VehicleInput.IMC_VehicleInput" 0 "(bIgnoreAllPressedKeysUntilRelease=True,bForceImmediately=False,bNotifyUserSettings=False)"))

(fn ConstructionScript)