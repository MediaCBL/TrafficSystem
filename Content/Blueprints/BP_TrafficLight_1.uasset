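; BP_TrafficLight_1 is a traffic light that recolours its point light when its signal state changes.
; On BeginPlay it binds a handler to the signal-changed event.
; The handler maps vehicle and pedestrian states to red, yellow or green, with Walk sharing green and Don't Walk sharing red, then applies that colour to the PointLight component.
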(event Custom|SignalChanged
  (params (Signal :type Traffic%20Signal%20Actor%20Object%20Reference) (NewState :type ETrafficSignalState%20Enum :default "Red"))
  (switch Utilities|FlowControl|Switch|SwitchonETrafficSignalState NewState
    (:Red
      (Variables|Default|SetLightColor "(R=1.000000,G=0.000000,B=0.000000,A=1.000000)"))
    (:Yellow
      (Variables|Default|SetLightColor "(R=0.924905,G=1.000000,B=0.000000,A=1.000000)"))
    (:Green
      (Variables|Default|SetLightColor "(R=0.000000,G=1.000000,B=0.000000,A=1.000000)"))
    (:Walk
      (Variables|Default|SetLightColor "(R=0.000000,G=1.000000,B=0.000000,A=1.000000)"))
    (:DontWalk
      (Variables|Default|SetLightColor "(R=1.000000,G=0.000000,B=0.000000,A=1.000000)")))
  (Rendering|Components|Light|SetLightColor (Variables|Default|GetPointLight) (Variables|Default|GetLightColor) true))

(event EventBeginPlay
  (EventDispatchers|BindEventtoOnSignalChanged (delegate Custom|SignalChanged)))

(fn ConstructionScript
  (|CallParentFunction))